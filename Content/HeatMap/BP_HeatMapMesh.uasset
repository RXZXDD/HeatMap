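; Heat map mesh actor that displays render target data on a static mesh through a dynamic material instance.
; The construction script creates the material and binds its Data texture to the assigned RT, or to one created from RTSetting.
; Events rebind Data to a newly created target, switch the Channel vector parameter, and call DoRenderHeatMap, which passes InParams and RT_HeatMap to the render function.
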(event `/HeatMap/HeatMap/BI_HeatMapInteract.UpdateRTSetting`
  (params (NewRTSetting :type "/HeatMap/HeatMap/S_RTSetting Structure"))
  (`self.DIM_HeatMapMaterial`
    (:`then`
      (bind _returnvalue (`KismetRenderingLibrary.CreateRenderTarget2D` NewRTSetting_X_5_F15F829049A9DD70C2C35CBCD9DDB927 NewRTSetting_Y_6_D6F045CA496FDBAEE7CF9E9DFB14A5EF NewRTSetting_Format_14_053B905D4D1BD2C30DB218A881B76ECD NewRTSetting_ClearColor_8_865E94A340F18F9824E16CB390F712E0))
      (`MaterialInstanceDynamic.SetTextureParameterValue` (`self.DIM_HeatMapMaterial`) "Data" _returnvalue))
    (:`else`)))

(event `/HeatMap/HeatMap/BI_HeatMapInteract.SwitchChannel`
  (params (NewChannel :type "/HeatMap/HeatMap/E_HeatMapDataChannel Enum" :default "NewEnumerator0"))
  (`MaterialInstanceDynamic.SetVectorParameterValue` (`self.DIM_HeatMapMaterial`) "Channel" (select `/HeatMap/HeatMap/E_HeatMapDataChannel` NewChannel :`NewEnumerator0` (struct :`A` 1.0) :`NewEnumerator1` (struct :`R` 1.0 :`A` 1.0) :`NewEnumerator2` (struct :`G` 1.0 :`A` 1.0) :!type "LinearColor Structure")))

(event `/HeatMap/HeatMap/BI_HeatMapInteract.DoRenderHeatMap`
  (`HeatMapBPLibrary.DoRenderHeatMap` "/HeatMap/HeatMap/RT_HeatMap.RT_HeatMap" (`self.In Params`)))

(fn `UserConstructionScript`
  (bind (_rtsetting_x _rtsetting_y _rtsetting_clearcolor _rtsetting_format) (break `/HeatMap/HeatMap/S_RTSetting` (`self.RTSetting`)))
  (bind _returnvalue (`PrimitiveComponent.CreateDynamicMaterialInstance` (`self.StaticMeshComponent`) 0 (`self.HeatMapMaterial`) "None"))
  (set `self.DIM_HeatMapMaterial` _returnvalue)
  (`|ExecutionSequence`
    (:`then_0`
      ;[1 1 1] RT
      (bind _rt (`self.RT`)
        (:`then`
          (`MaterialInstanceDynamic.SetTextureParameterValue` (`self.DIM_HeatMapMaterial`) "Data" _rt))
        (:`else`
          (bind _returnvalue_2 (`KismetRenderingLibrary.CreateRenderTarget2D` _rtsetting_x _rtsetting_y _rtsetting_format _rtsetting_clearcolor))
          (`MaterialInstanceDynamic.SetTextureParameterValue` (`self.DIM_HeatMapMaterial`) "Data" _returnvalue_2))))))